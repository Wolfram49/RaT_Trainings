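; Squad ruleset that builds caster kill-feed entries for wounds, team wounds, self-wounds, revives and vehicle destruction.
; Damage delegates, bound at player spawn and on seat changes, cache weapon icons per victim from the damage causer, its owner or seat weapon, with mine, C4 and cross fallbacks.
; Game events combine the cached icon, or a revive or suicide icon, with names, teams and role icons, then forward it to the caster GameState.
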(event `self.PostPlayerSpawn`
  (params (SpawningSoldier :type "SQSoldier Object Reference"))
  (`parent.PostPlayerSpawn` SpawningSoldier)
  (add `self.OnTakeAnyDamage` SpawningSoldier (`|CreateDelegate` :!event `Kill Death Ruleset Infantry`))
  (add `SQSoldier.OnChangedSeat` SpawningSoldier (`|CreateDelegate` :!event `CustomEvent_1`)))

(event `KillFeed_Sent`
  (bind _ascaster_game_state_squad_child (cast `/RaT_Trainings/Settings/Blueprints/Caster_GameStateSquad_Child` (`GameplayStatics.GetGameState`)))
  (`/RaT_Trainings/Settings/Blueprints/Caster_GameStateSquad_Child.Caster_OnKillFeedItemSendToGS_Event` _ascaster_game_state_squad_child (`self.Inst Text`) (`self.InstTeam`) (`self.Vict Text`) (`self.VictTeam`) (`self.Weapon_Texture`) (`self.InsRole`) (`self.VictRole`)))

(event `self.PlayerRevived`
  (params (Reviver :type "SQPlayerController Object Reference") (RevivedPlayer :type "SQPlayerController Object Reference"))
  ;[0.0582 1 0.05294] Revive Logic
  (`parent.PlayerRevived` Reviver RevivedPlayer)
  (set `self.Kill Feed ENUM` "NewEnumerator1")
  (`self.PlayerStateSetup` Reviver RevivedPlayer)
  (`self.TextureSetup` null))

(event `self.PlayerSelfWound`
  (params (Victim :type "SQPlayerController Object Reference"))
  ;[1 1 1] Incap/Knock Event Logic
  (`parent.PlayerSelfWound` Victim)
  (set `self.Kill Feed ENUM` "NewEnumerator2")
  (`self.PlayerStateSetup` Victim Victim)
  (`self.TextureSetup` Victim))

(event `self.PlayerWounded`
  (params (Killer :type "SQPlayerController Object Reference") (Victim :type "SQPlayerController Object Reference"))
  ;[1 1 1] Incap/Knock Event Logic
  (`parent.PlayerWounded` Killer Victim)
  (set `self.Kill Feed ENUM` "NewEnumerator0")
  (`self.PlayerStateSetup` Killer Victim)
  (`self.TextureSetup` Victim))

(event `self.PlayerTeamWounded`
  (params (Killer :type "SQPlayerController Object Reference") (Victim :type "SQPlayerController Object Reference"))
  ;[1 1 1] Incap/Knock Event Logic
  (`parent.PlayerTeamWounded` Killer Victim)
  (set `self.Kill Feed ENUM` "NewEnumerator0")
  (`self.PlayerStateSetup` Killer Victim)
  (`self.TextureSetup` Victim))

(event `self.VehicleDestroyed`
  (params (Killer :type "SQPlayerController Object Reference") (Victim :type "SQPlayerController Object Reference") (DestroyedVehicle :type "SQVehicle Object Reference"))
  (bind _vicdamagecauser (`self.VicDamageCauser`))
  ;[1 0.4716 0.4018] Vehicle
  (`parent.VehicleDestroyed` Killer Victim DestroyedVehicle)
  (bind _assqplayer_state (cast `SQPlayerState` (`Controller.PlayerState` (`Pawn.LastHitBy` DestroyedVehicle))))
  (set `self.Inst PS` _assqplayer_state)
  (set `self.Inst Text` (`KismetTextLibrary.Conv_StringToText` (`SQPlayerState.GetFullPlayerName` (`self.Inst PS`) false)))
  (bind _asbp_sqrole_settings (cast `/Game/Settings/Roles/BP_SQRoleSettings` (`SQPlayerState.GetCurrentRole` (`self.Inst PS`))))
  (set `self.InsRole` (`|ConvertAsset` (`.UI_Icon_27_CEC409E14C155F9F18EC1C961848686E` (break `/Game/Settings/Roles/FSQRoleEntry` (`.RoleEntry` (`/Game/Settings/Roles/BP_SQRoleSettings.GetRoleEntry` _asbp_sqrole_settings))))))
  (set `self.Weapon_Texture` (`BlueprintMapLibrary.Map_Find` _vicdamagecauser DestroyedVehicle))
  (`BlueprintMapLibrary.Map_Remove` _vicdamagecauser DestroyedVehicle)
  (set `self.VictTeam` (`SQTeamInterface.GetTeamId` DestroyedVehicle))
  (set `self.InstTeam` (`SQTeamState.Id` (`SQPlayerState.TeamState` (`self.Inst PS`))))
  (set `self.VictRole` (`SQVehicleUIStaticDataAsset.MapIcon` (`SQVehicle.StaticUIData` DestroyedVehicle)))
  (set `self.Vict Text` (`.DisplayName` (break `SQUsableData` (`SQVehicle.UsableData` DestroyedVehicle))))
  (`self.KillFeed_Sent`))

(event `VicTakeAnyDamage` :!signature `self.OnTakeAnyDamage`
  (params (DamagedActor :type "Actor Object Reference") (Damage :type "Float (single-precision)") (DamageType :type "DamageType Object Reference") (InstigatedBy :type "Controller Object Reference") (DamageCauser :type "Actor Object Reference"))
  (bind _assqvehicle (cast `SQVehicle` DamagedActor :!pure true))
  (bind _hudselectedtexture (`SQEquipableItem.HUDSelectedTexture` (`SQPawnInventoryComponent.CurrentWeapon` (`SQVehicleSeatComponent.GetSeatPawnInventory` (`SQPlayerController.GetCurrentSeat` (cast `SQPlayerController` (`Pawn.GetController` (`Actor.Instigator` DamageCauser)) :!pure true))))))
  ;[1 0.4716 0.4018] Vehicle
  (if (not (< Damage 3.0))
    (bind _assqequipable_item (cast `SQEquipableItem` DamageCauser)
      (:`then`
        (`BlueprintMapLibrary.Map_Add` (`self.VicDamageCauser`) _assqvehicle (`SQEquipableItem.HUDSelectedTexture` _assqequipable_item)))
      (:`CastFailed`
        (bind _assqequipable_item_2 (cast `SQEquipableItem` (`self.GetOwner` DamageCauser))
          (:`then`
            (`BlueprintMapLibrary.Map_Add` (`self.VicDamageCauser`) _assqvehicle (`SQEquipableItem.HUDSelectedTexture` _assqequipable_item_2)))
          (:`CastFailed`
            (`/Engine/EditorBlueprintResources/StandardMacros.IsValid` _hudselectedtexture
              (:`Is Valid`
                (`BlueprintMapLibrary.Map_Add` (`self.VicDamageCauser`) _assqvehicle _hudselectedtexture))
              (:`Is Not Valid`
                (cast `/Game/Blueprints/Items/EquippableItems/Handheld_Deployables/BP_Deployable_GenericMine_AT` DamageCauser
                  (:`then`
                    (`BlueprintMapLibrary.Map_Add` (`self.VicDamageCauser`) _assqvehicle "/Game/UI/HUD/Inventory/Weapons/Equipment/tm62_mine.tm62_mine"))
                  (:`CastFailed`
                    (cast `/Game/Blueprints/Items/EquippableItems/Handheld_Deployables/BP_Deployable_GenericExplosives` DamageCauser
                      (:`then`
                        (`BlueprintMapLibrary.Map_Add` (`self.VicDamageCauser`) _assqvehicle "/Game/UI/HUD/Inventory/Weapons/Equipment/T_m112_c4explosive_remote.T_m112_c4explosive_remote"))
                      (:`CastFailed`
                        (`BlueprintMapLibrary.Map_Add` (`self.VicDamageCauser`) _assqvehicle "/Game/UI/Widgets/Menu_Main/Icons/cross.cross")))))))))))))

(event `CustomEvent_1`
  (params (Soldier :type "SQSoldier Object Reference") (FromSeat :type "SQVehicleSeatComponent Object Reference") (ToSeat :type "SQVehicleSeatComponent Object Reference"))
  ;[1 0.4716 0.4018] Vehicle
  (if (`SQSoldier.IsInVehicle` Soldier)
    (add `self.OnTakeAnyDamage` (`SQSoldier.GetCurrentVehicle` Soldier) (`|CreateDelegate` :!event `VicTakeAnyDamage`))))

(fn `Kill Death Ruleset Infantry`
  (params (DamagedActor :type "Actor Object Reference") (Damage :type "Float (single-precision)") (DamageType :type "DamageType Object Reference") (InstigatedBy :type "Controller Object Reference") (DamageCauser :type "Actor Object Reference"))
  (bind _instigator (`Actor.Instigator` DamageCauser))
  (bind _returnvalue (`Pawn.GetController` _instigator))
  (bind _assqplayer_controller (cast `SQPlayerController` (`Pawn.GetController` (`Actor.Instigator` DamagedActor)) :!pure true))
  (bind _hudselectedtexture (`SQEquipableItem.HUDSelectedTexture` (`SQPawnInventoryComponent.CurrentWeapon` (`SQVehicleSeatComponent.GetSeatPawnInventory` (`SQPlayerController.GetCurrentSeat` (cast `SQPlayerController` _returnvalue :!pure true))))))
  (`/Engine/EditorBlueprintResources/StandardMacros.IsValid` DamageCauser
    (:`Is Valid`
      (bind _assqequipable_item (cast `SQEquipableItem` DamageCauser)
        (:`then`
          (`BlueprintMapLibrary.Map_Add` (`self.INFDamageCauser`) _assqplayer_controller (`SQEquipableItem.HUDSelectedTexture` _assqequipable_item)))
        (:`CastFailed`
          (bind _assqequipable_item_2 (cast `SQEquipableItem` (`self.GetOwner` DamageCauser))
            (:`then`
              (`BlueprintMapLibrary.Map_Add` (`self.INFDamageCauser`) _assqplayer_controller (`SQEquipableItem.HUDSelectedTexture` _assqequipable_item_2)))
            (:`CastFailed`
              (`/Engine/EditorBlueprintResources/StandardMacros.IsValid` _instigator
                (:`Is Valid`
                  (if (not (== InstigatedBy _returnvalue))
                    (`/Engine/EditorBlueprintResources/StandardMacros.IsValid` _hudselectedtexture
                      (:`Is Valid`
                        (`BlueprintMapLibrary.Map_Add` (`self.INFDamageCauser`) _assqplayer_controller _hudselectedtexture))
                      (:`Is Not Valid`
                        (cast `/Game/Blueprints/Items/EquippableItems/Handheld_Deployables/BP_Deployable_GenericMine_AT` DamageCauser :!label _label
                          (:`then`
                            (`BlueprintMapLibrary.Map_Add` (`self.INFDamageCauser`) _assqplayer_controller "/Game/UI/HUD/Inventory/Weapons/Equipment/tm62_mine.tm62_mine"))
                          (:`CastFailed`
                            (cast `/Game/Blueprints/Items/EquippableItems/Handheld_Deployables/BP_Deployable_GenericExplosives` DamageCauser
                              (:`then`
                                (`BlueprintMapLibrary.Map_Add` (`self.INFDamageCauser`) _assqplayer_controller "/Game/UI/HUD/Inventory/Weapons/Equipment/T_m112_c4explosive_remote.T_m112_c4explosive_remote"))
                              (:`CastFailed`
                                (`BlueprintMapLibrary.Map_Add` (`self.INFDamageCauser`) _assqplayer_controller "/Game/UI/Widgets/Menu_Main/Icons/cross.cross" :!label _label_2)))))))
                    (else
                      (goto _label))))
                (:`Is Not Valid`
                  (goto _label))))))))
    (:`Is Not Valid`
      (goto _label_2))))

(fn `PlayerStateSetup`
  (params (Target :type "Controller Object Reference") (Target1 :type "Controller Object Reference"))
  (`|ExecutionSequence`
    (:`then_0`
      (`/Engine/EditorBlueprintResources/StandardMacros.IsValid` Target
        (:`Is Valid`
          (bind _assqplayer_state (cast `SQPlayerState` (`Controller.PlayerState` Target))
            (:`then`
              (set `self.Inst PS` _assqplayer_state))
            (:`CastFailed`
              (set `self.Inst PS` null :!label _label))))
        (:`Is Not Valid`
          (goto _label))))
    (:`then_1`
      (`/Engine/EditorBlueprintResources/StandardMacros.IsValid` Target1
        (:`Is Valid`
          (bind _assqplayer_state_2 (cast `SQPlayerState` (`Controller.PlayerState` Target1))
            (:`then`
              (set `self.Vict PS` _assqplayer_state_2))
            (:`CastFailed`
              (set `self.Vict PS` null :!label _label_2))))
        (:`Is Not Valid`
          (goto _label_2))))))

(fn `TextureSetup`
  (params (InputPin :type "SQPlayerController Object Reference"))
  (bind _infdamagecauser (`self.INFDamageCauser`))
  (`|ExecutionSequence`
    (:`then_0`
      ;[1 0.1212 0.07146] Adding images for revive/suicide
      (switch `/RaT_Trainings/Settings/Blueprints/KillFeed/Caster_killFeedEnum` (`self.Kill Feed ENUM`)
        (:`NewEnumerator0`
          (set `self.Weapon_Texture` (`BlueprintMapLibrary.Map_Find` _infdamagecauser InputPin))
          (`BlueprintMapLibrary.Map_Remove` _infdamagecauser InputPin))
        (:`NewEnumerator1`
          (set `self.Weapon_Texture` "/Game/UI/Widgets/HUD/Scoreboard/ScoreboardTextures/ScoreboardRevive.ScoreboardRevive") ; Revive img
        )
        (:`NewEnumerator2`
          (set `self.Weapon_Texture` "/Game/UI/Widgets/HUD/Scoreboard/ScoreboardTextures/ScoreboardDeaths.ScoreboardDeaths") ; suicide(from fall)
        )))
    (:`then_1`
      ;[1 0.1818 0.98] Taking Roles to KillFeed
      (bind _inst_ps (`self.Inst PS`)
        (:`then`
          (bind _asbp_sqrole_settings (cast `/Game/Settings/Roles/BP_SQRoleSettings` (`SQPlayerState.GetCurrentRole` _inst_ps)))
          (set `self.InsRole` (`|ConvertAsset` (`.UI_Icon_27_CEC409E14C155F9F18EC1C961848686E` (break `/Game/Settings/Roles/FSQRoleEntry` (`.RoleEntry` (`/Game/Settings/Roles/BP_SQRoleSettings.GetRoleEntry` _asbp_sqrole_settings)))))))
        (:`else`)))
    (:`then_2`
      (bind _vict_ps (`self.Vict PS`)
        (:`then`
          (bind _asbp_sqrole_settings_2 (cast `/Game/Settings/Roles/BP_SQRoleSettings` (`SQPlayerState.GetCurrentRole` _vict_ps)))
          (set `self.VictRole` (`|ConvertAsset` (`.UI_Icon_27_CEC409E14C155F9F18EC1C961848686E` (break `/Game/Settings/Roles/FSQRoleEntry` (`.RoleEntry` (`/Game/Settings/Roles/BP_SQRoleSettings.GetRoleEntry` _asbp_sqrole_settings_2)))))))
        (:`else`)))
    (:`then_3`
      ;[1 1 1] Taking names for KillFeed
      (bind _inst_ps_2 (`self.Inst PS`)
        (:`then`
          (set `self.InstTeam` (`SQTeamState.Id` (`SQPlayerState.TeamState` _inst_ps_2))))
        (:`else`)))
    (:`then_4`
      (bind _vict_ps_2 (`self.Vict PS`)
        (:`then`
          (set `self.VictTeam` (`SQTeamState.Id` (`SQPlayerState.TeamState` _vict_ps_2))))
        (:`else`)))
    (:`then_5`
      (bind _inst_ps_3 (`self.Inst PS`)
        (:`then`
          (set `self.Inst Text` (`KismetTextLibrary.Conv_StringToText` (`SQPlayerState.GetFullPlayerName` _inst_ps_3 false))))
        (:`else`)))
    (:`then_6`
      (bind _vict_ps_3 (`self.Vict PS`)
        (:`then`
          (set `self.Vict Text` (`KismetTextLibrary.Conv_StringToText` (`SQPlayerState.GetFullPlayerName` _vict_ps_3 false))))
        (:`else`)))
    (:`then_7`
      (`self.KillFeed_Sent`))))

(fn `UserConstructionScript`
  (`parent.UserConstructionScript`))